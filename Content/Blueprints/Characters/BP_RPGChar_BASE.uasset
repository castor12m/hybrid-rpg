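; Base RPG character Blueprint that can be interacted with to open dialogue.
; On BeginPlay it turns off the dialogue indicator's shadow and caches the GM_RPG game mode.
; Interact puts both the instigator and itself into interaction, locking and halting its own movement component, then shows dialogue through the game mode's HUD widget and prints a hardcoded welcome line.
; FinishInteraction clears its interaction lock.
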(event `self.ReceiveBeginPlay`
  (`PrimitiveComponent.SetCastShadow` (`self.DialogueIndicator`) false)
  (bind _asgm_rpg (cast `/Game/Blueprints/GM_RPG` (`GameplayStatics.GetGameMode`)))
  (set `self.GameMode` _asgm_rpg))

(event `/Game/Blueprints/Interfaces/BPI_Interaction.Interact`
  (params (Instigator :type "/Game/Blueprints/Characters/BP_RPGChar_BASE Object Reference"))
  (`self.StartInteraction` Instigator)
  (`self.StartInteraction`)
  (bind _dialogue (`self.ShowDialogueLine`))
  (`KismetSystemLibrary.PrintString` _dialogue))

(event `/Game/Blueprints/Interfaces/BPI_Interaction.FinishInteraction`
  (`self.EndInteraction`))

(fn `EndInteraction`
  (set `self.IsInteractionLocked` false))

(fn `ShowDialogueLine`
  (returns (Dialogue :type String))
  (`/Game/Widgets/WBP_HUD.ShowDialogue` (`/Game/Blueprints/GM_RPG.HUDWidget` (`self.GameMode`)) self)
  (return "Welcom to our city"))

(fn `StartInteraction`
  (set `self.IsInteractionLocked` true)
  (`MovementComponent.StopMovementImmediately` (`self.CharacterMovement`)))

(fn `UserConstructionScript`)